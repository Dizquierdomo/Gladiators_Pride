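; Minotaur enemy character that fights the Gladiator player, with its own health bar and an end-game call on death.
; On BeginPlay it binds the health bar, toggles low-attack FX visibility, socket-attaches its weapon and disables attack overlaps.
; Player weapon overlaps deal damage once per attack ID, while skill hits only print a stun message.
; Low-attack overlaps damage a non-jumping Gladiator, then switch themselves off.
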(event OnComponentBeginOverlap(CapsuleComponent)
  (params (OverlappedComponent :type Primitive%20Component%20Object%20Reference) (OtherActor :type Actor%20Object%20Reference) (OtherComp :type Primitive%20Component%20Object%20Reference) (OtherBodyIndex :type Integer) (bFromSweep :type Boolean) (SweepResult :type Hit%20Result%20Structure%20%28by%20ref%29))
  ;[1 0.277 0.9252] Damage Taked Control
  (if (Components|ComponentHasTag OtherComp "player.weapon")
    (bind _asweapon (Utilities|Casting|CastToWeapon OtherActor))
    (bind _returnvalue (Class|Weapon|GetAttackID _asweapon))
    (if (!= _returnvalue (Variables|Default|GetLastPlayerAttackID))
      (Variables|Default|SetLastPlayerAttackID _returnvalue)
      (CallFunction|TakeDamage (Variables|/Script/UnrealEngine_5_1_0.Weapon|GetAtkValue _asweapon)))
    (elif (Components|ComponentHasTag OtherComp "player.skill")
      (Development|PrintString "STUN!!!"))))

(event OnComponentBeginOverlap(LowAtkCollision)
  (params (OverlappedComponent :type Primitive%20Component%20Object%20Reference) (OtherActor :type Actor%20Object%20Reference) (OtherComp :type Primitive%20Component%20Object%20Reference) (OtherBodyIndex :type Integer) (bFromSweep :type Boolean) (SweepResult :type Hit%20Result%20Structure%20%28by%20ref%29))
  ;[1 0.2048 0] Low Attack
  (if (Components|ComponentHasTag OtherComp "player.hitBox")
    (bind _asgladiator_bp (Utilities|Casting|CastToGladiator_BP OtherActor))
    (if (not (Variables|/Script/UnrealEngine_5_1_0.Gladiator|GetIsJumping _asgladiator_bp))
      (Default|TakeDamage _asgladiator_bp (Variables|Default|GetLowAtkDamage))
      (Variables|/Script/Engine.PrimitiveComponent|SetbGenerateOverlapEvents (Variables|Default|GetLowAtkCollision) false))))

(event Custom|TakeDamage
  (params (DamageValue :type Integer))
  (bind _self self)
  ;[1 0.125 0.125] Take Damage
  (bind _returnvalue (Class|GameCharacter|GetHealthPoints _self))
  (Class|GameCharacter|SetHealthPoints _self (- _returnvalue DamageValue))
  (bind _returnvalue_2 (Class|GameCharacter|GetHealthPoints))
  (if (<= _returnvalue_2 0)
    (Default|CallEndGame self)))

(event Custom|BindPlayerCharacterToStatusBars
  ;[1 0.8143 0.2855] Bind Player Character To Status Bars
  (bind _asenemy_health_bar (Utilities|Casting|CastToEnemyHealthBar (UserInterface|GetWidget (Variables|Default|GetEnemyHealthBar))))
  (Variables|/Game/Widgets/EnemyHealthBar.EnemyHealthBar_C|SetGameCharacter _asenemy_health_bar self))

(event EventBeginPlay
  (CallFunction|BindPlayerCharactertoStatusBars)
  (bind _aslow_atk_fx (Utilities|Casting|CastToLowAtkFX (Utilities|Array|Get(acopy) (Actor|GetAllChildActors true))))
  (Rendering|ToggleVisibility (Variables|/Game/Blueprints/LowAtkFX.LowAtkFX_C|GetDefaultSceneRoot _aslow_atk_fx) true)
  (Variables|/Script/Engine.PrimitiveComponent|SetbGenerateOverlapEvents (Variables|Default|GetLowAtkCollision) false)
  (bind _outactors (Actor|GetAllActorsOfClass "/Game/Blueprints/EnemyWeapon_BP.EnemyWeapon_BP_C"))
  (if (== (Utilities|Array|Length _outactors) 1)
    (bind _output_get (Variables|Default|SetWeapon (Utilities|Array|Get(acopy) _outactors)))
    (Transformation|AttachComponentToComponent _output_get (Variables|Character|GetMesh) "WeaponSocket" "SnapToTarget" "SnapToTarget" "SnapToTarget" false)
    (Variables|/Script/Engine.PrimitiveComponent|SetbGenerateOverlapEvents (Variables|/Script/UnrealEngine_5_1_0.Weapon|GetWeaponCollision (Variables|Default|GetWeapon)) false)))

(fn ConstructionScript)