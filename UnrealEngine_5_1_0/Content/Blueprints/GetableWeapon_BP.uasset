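; GetableWeapon_BP is a weapon pickup that shows its Item's mesh and hands that Item to the player's inventory.
; A sphere overlap with the tagged player hitbox sets an in-range flag.
; On the Gladiator's GetWeapon event, an in-range pickup moves the Item to world origin and calls AddToInventory on the player's inventory component.
; It destroys itself and prints the result, even when the add fails.
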(event OnComponentBeginOverlap(Sphere)
  (params (OverlappedComponent :type Primitive%20Component%20Object%20Reference) (OtherActor :type Actor%20Object%20Reference) (OtherComp :type Primitive%20Component%20Object%20Reference) (OtherBodyIndex :type Integer) (bFromSweep :type Boolean) (SweepResult :type Hit%20Result%20Structure%20%28by%20ref%29))
  (if (Components|ComponentHasTag OtherComp "player.hitBox")
    (Variables|Default|SetIsPlayerInRange true)))

(event OnComponentEndOverlap(Sphere)
  (params (OverlappedComponent :type Primitive%20Component%20Object%20Reference) (OtherActor :type Actor%20Object%20Reference) (OtherComp :type Primitive%20Component%20Object%20Reference) (OtherBodyIndex :type Integer))
  (if (Components|ComponentHasTag OtherComp "player.hitBox")
    (Variables|Default|SetIsPlayerInRange false)))

(event Custom|GoToPlayerInventory
  (bind _item (Variables|Default|GetItem))
  (if (Variables|Default|GetIsPlayerInRange)
    (bind _asgladiator_bp (Utilities|Casting|CastToGladiator_BP (Game|GetPlayerCharacter 0)))
    (Transformation|SetActorLocation _item "0, 0, 0" false false)
    (bind _result (Default|AddtoInventory (Actor|GetComponentbyClass _asgladiator_bp "/Game/Blueprints/Inventory_Component.Inventory_Component_C") _item (Variables|Default|GetIndex)))
    (switch int _result
      (:-1
        (Actor|DestroyActor)
        (Development|PrintString "ERROR" true true "(R=0.526042,G=0.000000,B=0.004525,A=1.000000)"))
      (:0
        (Actor|DestroyActor)
        (Development|PrintString "ItemNotAdded" true true "(R=0.481278,G=0.000000,B=1.000000,A=1.000000)"))
      (:1
        (Actor|DestroyActor)
        (Development|PrintString "ItemAdded" true true "(R=0.032721,G=0.505208,B=0.000000,A=1.000000)")))))

(event EventBeginPlay
  (bind _asgladiator_bp (Utilities|Casting|CastToGladiator_BP (Game|GetPlayerCharacter 0)))
  (EventDispatchers|BindEventtoGetWeapon _asgladiator_bp (delegate Custom|GoToPlayerInventory))
  (Components|StaticMesh|SetStaticMesh (Variables|Default|GetWeaponMesh) (Variables|/Script/Engine.StaticMeshComponent|GetStaticMesh (Variables|/Script/UnrealEngine_5_1_0.Weapon|GetWeaponMesh (Variables|Default|GetItem)))))

(event Collision|EventActorBeginOverlap
  (params (OtherActor :type Actor%20Object%20Reference)))

(event EventTick
  (params (DeltaSeconds :type Float%20%28single-precision%29)))

(fn ConstructionScript)