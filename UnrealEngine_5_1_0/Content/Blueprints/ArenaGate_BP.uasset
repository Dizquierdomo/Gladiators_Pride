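; ArenaGate_BP is an arena gate that opens through a Level Sequence when the player's get-weapon event fires nearby.
; DistanceTrigger tracks whether a component tagged as the player hit box is in range.
; BeginPlay binds OpenGate to the Gladiator_BP get-weapon event and creates the OpenArenaGates sequence player.
; OpenGate checks the range flag, then disables the trigger's overlaps, clears the flag and plays the sequence, so it opens only once.
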(event OnComponentBeginOverlap(DistanceTrigger)
  (params (OverlappedComponent :type Primitive%20Component%20Object%20Reference) (OtherActor :type Actor%20Object%20Reference) (OtherComp :type Primitive%20Component%20Object%20Reference) (OtherBodyIndex :type Integer) (bFromSweep :type Boolean) (SweepResult :type Hit%20Result%20Structure%20%28by%20ref%29))
  (if (Components|ComponentHasTag OtherComp "player.hitBox")
    (Variables|Default|SetIsPlayerInRange true)))

(event OnComponentEndOverlap(DistanceTrigger)
  (params (OverlappedComponent :type Primitive%20Component%20Object%20Reference) (OtherActor :type Actor%20Object%20Reference) (OtherComp :type Primitive%20Component%20Object%20Reference) (OtherBodyIndex :type Integer))
  (if (Components|ComponentHasTag OtherComp "player.hitBox")
    (Variables|Default|SetIsPlayerInRange false)))

(event Custom|OpenGate
  (if (Variables|Default|GetIsPlayerInRange)
    (Variables|/Script/Engine.PrimitiveComponent|SetbGenerateOverlapEvents (Variables|Default|GetDistanceTrigger) false)
    (Variables|Default|SetIsPlayerInRange false)
    (Sequencer|Player|Play (Variables|/Script/LevelSequence.LevelSequenceActor|GetSequencePlayer (Variables|Default|GetGatesAnimation)) :!class /Script/MovieScene.MovieSceneSequencePlayer)))

(event EventBeginPlay
  (bind _asgladiator_bp (Utilities|Casting|CastToGladiator_BP (Game|GetPlayerCharacter 0)))
  (EventDispatchers|BindEventtoGetWeapon _asgladiator_bp (delegate Custom|OpenGate))
  (bind _outactor (Sequencer|Player|CreateLevelSequencePlayer "/Game/Animations/OpenArenaGates.OpenArenaGates"))
  (Variables|Default|SetGatesAnimation _outactor))

(event Collision|EventActorBeginOverlap
  (params (OtherActor :type Actor%20Object%20Reference)))

(event EventTick
  (params (DeltaSeconds :type Float%20%28single-precision%29)))

(fn ConstructionScript)