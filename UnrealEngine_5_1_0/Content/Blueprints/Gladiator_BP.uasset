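; Playable gladiator character that spawns a sword on its weapon socket and handles movement, camera, enemy targeting and attacks.
; Enhanced Input actions drive inherited or external movement and combat functions, with input disabled for the duration returned by each attack.
; A looping timer regenerates energy and refreshes the status bar.
; The TargetZone overlap tracks the enemy in range, calling TargetEnemy when an overlap ends.
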(event OnComponentBeginOverlap(TargetZone)
  (params (OverlappedComponent :type Primitive%20Component%20Object%20Reference) (OtherActor :type Actor%20Object%20Reference) (OtherComp :type Primitive%20Component%20Object%20Reference) (OtherBodyIndex :type Integer) (bFromSweep :type Boolean) (SweepResult :type Hit%20Result%20Structure%20%28by%20ref%29))
  (Class|Gladiator|SetEnemyinTargetRange OtherActor)
  (Utilities|Casting|CastToCharacter (Variables|Default|GetEnemyInTargetRange)
    (:then
      (Development|PrintString "InRange" true true "(R=0.000000,G=0.868849,B=1.000000,A=1.000000)"))
    (:CastFailed
      (Development|PrintString "OutOfRange" true true "(R=1.000000,G=0.000000,B=0.798049,A=1.000000)"))))

(event OnComponentEndOverlap(TargetZone)
  (params (OverlappedComponent :type Primitive%20Component%20Object%20Reference) (OtherActor :type Actor%20Object%20Reference) (OtherComp :type Primitive%20Component%20Object%20Reference) (OtherBodyIndex :type Integer))
  (Class|Gladiator|SetEnemyinTargetRange)
  (Class|Gladiator|TargetEnemy)
  (Utilities|Casting|CastToCharacter (Variables|Default|GetEnemyInTargetRange)
    (:then
      (Development|PrintString "InRange" true true "(R=0.000000,G=0.868849,B=1.000000,A=1.000000)"))
    (:CastFailed
      (Development|PrintString "OutOfRange" true true "(R=1.000000,G=0.000000,B=0.798049,A=1.000000)"))))

(event Custom|EnergyRegen
  (bind _returnvalue (Class|Gladiator|GetEnergyPoints))
  (bind _returnvalue_2 (Class|Gladiator|GetEnergyRecoveryPerSecond))
  (Class|Gladiator|SetEnergyPoints (+ _returnvalue (Math|Float|Truncate _returnvalue_2)))
  (CallFunction|UpdateEnergyBar (Variables|Default|GetStatusBars)))

(event Input|EnhancedActionEvents|EnhancedInputActionMoveForward_Input
  (params (ActionValue :type Float%20%28double-precision%29) (ElapsedSeconds :type Float%20%28double-precision%29) (TriggeredSeconds :type Float%20%28double-precision%29) (InputAction :type Input%20Action%20Object%20Reference :default "/Game/Inputs/MoveForward_Input.MoveForward_Input"))
  ;[1 0.6214 0.2247 1 20] Movement Control
  (:Triggered
    (Class|Gladiator|ForwardMove ActionValue))
  (:Completed
    (Variables|Default|SetIsWalkingForward false)
    (Variables|Default|SetIsWalkingBackward false)))

(event Input|EnhancedActionEvents|EnhancedInputActionMoveRight_Input
  (params (ActionValue :type Float%20%28double-precision%29) (ElapsedSeconds :type Float%20%28double-precision%29) (TriggeredSeconds :type Float%20%28double-precision%29) (InputAction :type Input%20Action%20Object%20Reference :default "/Game/Inputs/MoveRight_Input.MoveRight_Input"))
  ;[1 0.6214 0.2247 1 20] Movement Control
  (:Triggered
    (Class|Gladiator|RightMove ActionValue))
  (:Completed
    (Variables|Default|SetIsWalkingRight false)
    (Variables|Default|SetIsWalkingLeft false)))

(event Input|EnhancedActionEvents|EnhancedInputActionAttack_Input
  (params (ActionValue :type Boolean) (ElapsedSeconds :type Float%20%28double-precision%29) (TriggeredSeconds :type Float%20%28double-precision%29) (InputAction :type Input%20Action%20Object%20Reference :default "/Game/Inputs/Attack_Input.Attack_Input"))
  (bind _returnvalue (Game|GetPlayerController 0))
  (:Triggered
    (bind _returnvalue_2 (Class|Gladiator|WeaponAttack))
    (if (== (.atktime _returnvalue_2) -1.0)
      (Development|PrintString "Not Enougth Energy")
      (elif (== (.atktime _returnvalue_2) 0.0)
        (Development|PrintString "Weapon is needed for execute an atack")))
    (Input|DisableInput _returnvalue)
    (Utilities|FlowControl|Delay (.atktime _returnvalue_2))
    (Input|EnableInput _returnvalue)
    (Components|Animation|SetAnimationMode (Variables|Character|GetMesh) "AnimationBlueprint")
    (CallFunction|UpdateEnergyBar (Variables|Default|GetStatusBars))))

(event Input|EnhancedActionEvents|EnhancedInputActionRotateCameraX_Input
  (params (ActionValue :type Float%20%28double-precision%29) (ElapsedSeconds :type Float%20%28double-precision%29) (TriggeredSeconds :type Float%20%28double-precision%29) (InputAction :type Input%20Action%20Object%20Reference :default "/Game/Inputs/RotateCameraX_Input.RotateCameraX_Input"))
  ;[0.2061 0.3129 1 1 20] Camera Control
  (:Triggered
    (Pawn|Input|AddControllerYawInput ActionValue)))

(event Input|EnhancedActionEvents|EnhancedInputActionRotateCameraY_Input
  (params (ActionValue :type Float%20%28double-precision%29) (ElapsedSeconds :type Float%20%28double-precision%29) (TriggeredSeconds :type Float%20%28double-precision%29) (InputAction :type Input%20Action%20Object%20Reference :default "/Game/Inputs/RotateCameraY_Input.RotateCameraY_Input"))
  ;[0.2061 0.3129 1 1 20] Camera Control
  (:Triggered
    (Pawn|Input|AddControllerPitchInput ActionValue)))

(event Input|EnhancedActionEvents|EnhancedInputActionTargetEnemy_Input
  (params (ActionValue :type Boolean) (ElapsedSeconds :type Float%20%28double-precision%29) (TriggeredSeconds :type Float%20%28double-precision%29) (InputAction :type Input%20Action%20Object%20Reference :default "/Game/Inputs/TargetEnemy_Input.TargetEnemy_Input"))
  (:Triggered
    (Class|Gladiator|TargetEnemy)))

(event EventBeginPlay
  (Utilities|Time|SetTimerbyEvent (delegate Custom|EnergyRegen) 1.0 true)
  (bind _returnvalue (Game|SpawnActorfromClass "/Game/Blueprints/Gladiator_Sword_BP.Gladiator_Sword_BP_C" (Transformation|GetSocketTransform (Variables|Character|GetMesh) "WeaponSocket" "RTS_World") "Undefined" 0 0))
  (Variables|Default|SetWeapon _returnvalue)
  (Transformation|AttachComponentToComponent _returnvalue (Variables|Character|GetMesh) "WeaponSocket" "SnapToTarget" "SnapToTarget" "SnapToTarget" true))

(event Collision|EventActorBeginOverlap
  (params (OtherActor :type Actor%20Object%20Reference)))

(event EventTick
  (params (DeltaSeconds :type Float%20%28single-precision%29)))

(event EventPossessed
  (params (NewController :type Controller%20Object%20Reference))
  ;[0.2448 0.2448 0.2448 1 20] Bind Inputs
  (bind _asplayer_controller (Utilities|Casting|CastToPlayerController NewController))
  (Input|AddMappingContext (PlayerController|LocalPlayerSubsystems|GetEnhancedInputLocalPlayerSubsystem _asplayer_controller) "/Game/Inputs/Arena_Context.Arena_Context" 0 "(bIgnoreAllPressedKeysUntilRelease=True,bForceImmediately=False)"))

(fn ConstructionScript)

(fn UpdateEnergyBar
  (params (GladiatorStatus_BP :type Gladiator%20Status%20Object%20Reference))
  (if (Utilities|IsValid GladiatorStatus_BP)
    (Default|EnergyBarUpdate GladiatorStatus_BP)))